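; Side-scroller platform that moves when the player character enters its Box trigger and travels back when they leave.
; Overlap begin and end play and reverse the MPF timeline, which drives MovingPlatform's relative location without sweep.
; Each timeline update also applies a blue material, including during reversal.
; After the player exits, a PlayerMPF flag makes Tick reapply CubeMaterial every frame until re-entry.
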(event OnComponentBeginOverlap(Box)
  (params (OverlappedComponent :type Primitive%20Component%20Object%20Reference) (OtherActor :type Actor%20Object%20Reference) (OtherComp :type Primitive%20Component%20Object%20Reference) (OtherBodyIndex :type Integer) (bFromSweep :type Boolean) (SweepResult :type Hit%20Result%20Structure%20%28by%20ref%29))
  (Utilities|Casting|CastToSideScrollerCharacter OtherActor)
  (Variables|Default|SetPlayer_MPF false)
  (bind _movingplatform_z (Timeline|MPF Play)
    (:Update
      (Transformation|SetRelativeLocation (Variables|Default|GetMovingPlatform) _movingplatform_z false false)
      (Rendering|Material|SetMaterial (Variables|Default|GetMovingPlatform) 0 "/Game/VFX/blue.blue"))))

(event OnComponentEndOverlap(Box)
  (params (OverlappedComponent :type Primitive%20Component%20Object%20Reference) (OtherActor :type Actor%20Object%20Reference) (OtherComp :type Primitive%20Component%20Object%20Reference) (OtherBodyIndex :type Integer))
  (Utilities|Casting|CastToSideScrollerCharacter OtherActor)
  (Variables|Default|SetPlayer_MPF true)
  (bind _movingplatform_z (Timeline|MPF Reverse)
    (:Update
      (Transformation|SetRelativeLocation (Variables|Default|GetMovingPlatform) _movingplatform_z false false)
      (Rendering|Material|SetMaterial (Variables|Default|GetMovingPlatform) 0 "/Game/VFX/blue.blue"))))

(event EventBeginPlay)

(event Collision|EventActorBeginOverlap
  (params (OtherActor :type Actor%20Object%20Reference)))

(event EventTick
  (params (DeltaSeconds :type Float%20%28single-precision%29))
  (if (Variables|Default|GetPlayer_MPF)
    (Rendering|Material|SetMaterial (Variables|Default|GetMovingPlatform) 0 "/Game/SideScrollerBP/Meshes/CubeMaterial.CubeMaterial")))

(fn ConstructionScript)